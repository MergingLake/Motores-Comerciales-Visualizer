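; BP_Car is the car actor for a product visualizer, offering UI-driven paint color changes, toggleable rotation and mouse look.
; BeginPlay creates a dynamic material from the car paint master, spawns WBP_Interface with a visible cursor and adds the mouse-look input mapping.
; Widget events set both BaseColor and ChameleonColor to the chosen color and toggle the RotatingMovement component.
; The mouse-look action feeds controller yaw and pitch.
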(event `self.ReceiveBeginPlay`
  (bind _returnvalue (`GameplayStatics.GetPlayerController` 0))
  (bind _returnvalue_2 (`PrimitiveComponent.CreateDynamicMaterialInstance` (`self.MeshProduct`) 3 "/Game/Car5/Materials/Masters/M_CarPaint_Master.M_CarPaint_Master" "None"))
  (set `self.MID_Product` _returnvalue_2)
  (`EnhancedInputSubsystemInterface.AddMappingContext` (pcsubsystem `EnhancedInputLocalPlayerSubsystem` (`GameplayStatics.GetPlayerController` 0)) "/Game/Input/IMC_MouseLook.IMC_MouseLook" 0 (struct))
  (bind _returnvalue_3 (`|CreateWidget` "/Game/Visualizer/Widgets/WBP_Interface.WBP_Interface_C"))
  (bind _output_get (set `self.Ref_UI` _returnvalue_3))
  (`UserWidget.AddToViewport` _output_get 0)
  (set `PlayerController.bShowMouseCursor` true _returnvalue)
  (`WidgetBlueprintLibrary.SetInputMode_GameAndUIEx` _returnvalue null)
  (add `/Game/Visualizer/Widgets/WBP_Interface.ChangeProductColor` (`self.Ref_UI`) (delegate `UpdateProdColor`))
  (add `/Game/Visualizer/Widgets/WBP_Interface.SetRotation` (`self.Ref_UI`) (delegate `UpdateRotation`)))

(event `UpdateRotation`
  (params (RotationState :type Boolean))
  (`ActorComponent.SetActive` (`self.RotatingMovement`) RotationState false))

(event `UpdateProdColor`
  (params (NewColor :type "LinearColor Structure"))
  (`MaterialInstanceDynamic.SetVectorParameterValue` (`self.MID_Product`) "BaseColor" NewColor)
  (`MaterialInstanceDynamic.SetVectorParameterValue` (`self.MID_Product`) "ChameleonColor" NewColor))

(event `EnhancedInput|/Game/Input/Actions/IA_MouseLook`
  (params (ActionValue :type "Vector2D Structure") (ElapsedSeconds :type "Float (double-precision)") (TriggeredSeconds :type "Float (double-precision)") (InputAction :type "InputAction Object Reference" :default "/Game/Input/Actions/IA_MouseLook.IA_MouseLook"))
  (:`Triggered`
    (`self.AddControllerYawInput` ActionValue_X)
    (`self.AddControllerPitchInput` ActionValue_Y)))

(fn `UserConstructionScript`)