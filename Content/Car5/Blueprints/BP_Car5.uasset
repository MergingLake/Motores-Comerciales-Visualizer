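; BP_Car5 is a player-drivable car Blueprint controlled with keyboard and mouse.
; Hard-coded key events feed full-or-zero throttle, reverse and steering values to VehicleMovement, with W/S and A/D for driving and Space for the handbrake.
; Tick reads the mouse delta from player controller 0 to drive controller yaw and inverted pitch for looking around.
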(event `Key|W`
  (params (Key :type "Key Structure"))
  (bind _vehiclemovement (`self.VehicleMovement`))
  (:`Pressed`
    (`WheeledVehicleMovementComponent.SetThrottleInput` _vehiclemovement 1.0))
  (:`Released`
    (`WheeledVehicleMovementComponent.SetThrottleInput` _vehiclemovement 0.0)))

(event `Key|S`
  (params (Key :type "Key Structure"))
  (bind _vehiclemovement (`self.VehicleMovement`))
  (:`Pressed`
    (`WheeledVehicleMovementComponent.SetThrottleInput` _vehiclemovement -1.0))
  (:`Released`
    (`WheeledVehicleMovementComponent.SetThrottleInput` _vehiclemovement 0.0)))

(event `Key|D`
  (params (Key :type "Key Structure"))
  (bind _vehiclemovement (`self.VehicleMovement`))
  (:`Pressed`
    (`WheeledVehicleMovementComponent.SetSteeringInput` _vehiclemovement 1.0))
  (:`Released`
    (`WheeledVehicleMovementComponent.SetSteeringInput` _vehiclemovement 0.0)))

(event `Key|A`
  (params (Key :type "Key Structure"))
  (bind _vehiclemovement (`self.VehicleMovement`))
  (:`Pressed`
    (`WheeledVehicleMovementComponent.SetSteeringInput` _vehiclemovement -1.0))
  (:`Released`
    (`WheeledVehicleMovementComponent.SetSteeringInput` _vehiclemovement 0.0)))

(event `Key|SpaceBar`
  (params (Key :type "Key Structure"))
  (bind _vehiclemovement (`self.VehicleMovement`))
  (:`Pressed`
    (`WheeledVehicleMovementComponent.SetHandbrakeInput` _vehiclemovement true))
  (:`Released`
    (`WheeledVehicleMovementComponent.SetHandbrakeInput` _vehiclemovement false)))

(event `self.ReceiveTick`
  (params (DeltaSeconds :type "Float (single-precision)"))
  (bind (_deltax _deltay) (`PlayerController.GetInputMouseDelta` (`GameplayStatics.GetPlayerController` 0)))
  (`self.AddControllerYawInput` _deltax)
  (`self.AddControllerPitchInput` (* _deltay -1.0)))

(fn `UserConstructionScript`)